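; BP_Puzzl is a rotation puzzle that opens and closes a linked door (BpDoor).
; InteractwithPuzzle turns a piece left or right in yaw steps, then ChekCode compares that piece's yaw to its target in Code within a small tolerance.
; Results are stored per piece in CodeGood, and the door opens only when every entry is true.
; A Box overlap toggles player input and shows or clears a tutorial widget.
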(event OnComponentBeginOverlap(Box)
  (params (OverlappedComponent :type Primitive%20Component%20Object%20Reference) (OtherActor :type Actor%20Object%20Reference) (OtherComp :type Primitive%20Component%20Object%20Reference) (OtherBodyIndex :type Integer) (bFromSweep :type Boolean) (SweepResult :type Hit%20Result%20Structure%20%28by%20ref%29))
  (Input|EnableInput (Game|GetPlayerController 0))
  (bind _returnvalue (UserInterface|CreateWidget "/Game/LevelOnTheBrink/BP/Door_with_pazzell/Tutorial.Tutorial_C"))
  (UserInterface|Viewport|AddtoViewport _returnvalue 0))

(event OnComponentEndOverlap(Box)
  (params (OverlappedComponent :type Primitive%20Component%20Object%20Reference) (OtherActor :type Actor%20Object%20Reference) (OtherComp :type Primitive%20Component%20Object%20Reference) (OtherBodyIndex :type Integer))
  (Input|DisableInput (Game|GetPlayerController 0))
  (Viewport|RemoveAllWidgets))

(event EventInteractwithPuzzle
  (params (Component :type Primitive%20Component%20Object%20Reference) (RotateLeft :type Boolean))
  (CallFunction|Rotate Component RotateLeft))

(fn ConstructionScript)

(fn Rotate
  (params (Component :type Primitive%20Component%20Object%20Reference) (RotateLeft :type Boolean))
  ;[1 1 1] Фукция поворота пазла
  (if RotateLeft
    (Transformation|AddRelativeRotation Component (Math|Rotator|MakeRotator 0.0 0.0 (* (Variables|Default|GetRotateValue) -1.0)) false false)
    (else
      (Transformation|AddRelativeRotation Component (Math|Rotator|MakeRotator 0.0 0.0 (Variables|Default|GetRotateValue)) false false)))
  (Development|PrintString (Utilities|String|ToString(Rotator) (Variables|/Script/Engine.SceneComponent|GetRelativeRotation Component)))
  (CallFunction|ChekCode Component))

(fn ChekCode
  (params (Component :type Primitive%20Component%20Object%20Reference))
  (bind _bp_door (Variables|Default|GetBp_Door))
  ;[1 1 1] Проверяет, можем ли мы открыть дверь
  (if (== Component (Variables|Default|GetPuzzle))
    (LocalVariables|Setselectedmesh 0)
    (Utilities|Array|SetArrayElem (Variables|Default|GetCodeGood) (LocalVariables|Getselectedmesh) (Math|Float|NearlyEqual(Float) (Utilities|Array|Get(acopy) (Variables|Default|GetCode) (LocalVariables|Getselectedmesh)) (.yaw (Variables|/Script/Engine.SceneComponent|GetRelativeRotation Component)) 1.0) :!label _label)
    (bind _array_element (Utilities|Array|ForEachLoopwithBreak (Variables|Default|GetCodeGood) :!label _label_2)
      (:LoopBody
        (if (not _array_element)
          (LocalVariables|SetLocalFailed true)
          (goto _label_2 Break)))
      (:Completed
        (if (LocalVariables|GetLocalFailed)
          (Default|CloseDoor _bp_door)
          (else
            (Default|OpenDoor _bp_door)))))
    (elif (== Component (Variables|Default|GetPuzzle1))
      (LocalVariables|Setselectedmesh 1)
      (goto _label)
      (elif (== Component (Variables|Default|GetPuzzle2))
        (LocalVariables|Setselectedmesh 2)
        (goto _label)))))