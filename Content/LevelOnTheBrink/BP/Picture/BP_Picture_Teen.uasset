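; BP_Picture_Teen is an interactable picture that shows the Teen_WD widget when the player presses Interact nearby.
; Box overlap enables input, shows the Widget_INTERACT prompt and opens a gate that lets Interact through.
; A FlipFlop toggles the picture widget on and off.
; Leaving the box disables input and removes all widgets, without resetting the FlipFlop or closing the gate.
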(event OnComponentBeginOverlap(Box)
  (params (OverlappedComponent :type Primitive%20Component%20Object%20Reference) (OtherActor :type Actor%20Object%20Reference) (OtherComp :type Primitive%20Component%20Object%20Reference) (OtherBodyIndex :type Integer) (bFromSweep :type Boolean) (SweepResult :type Hit%20Result%20Structure%20%28by%20ref%29))
  (Input|EnableInput (Game|GetPlayerController 0))
  (bind _returnvalue (UserInterface|CreateWidget "/Game/LevelOnTheBrink/BP/UI/Widget_INTERACT.Widget_INTERACT_C"))
  (UserInterface|Viewport|AddtoViewport _returnvalue 0)
  (Utilities|FlowControl|Gate true) ; enters at Open
)

(event OnComponentEndOverlap(Box)
  (params (OverlappedComponent :type Primitive%20Component%20Object%20Reference) (OtherActor :type Actor%20Object%20Reference) (OtherComp :type Primitive%20Component%20Object%20Reference) (OtherBodyIndex :type Integer))
  (Input|DisableInput (Game|GetPlayerController 0))
  (Viewport|RemoveAllWidgets)
  (Widget|RemovefromParent (stale Input|ActionEvents|InputActionInteract _returnvalue)))

(event EventBeginPlay)

(event Collision|EventActorBeginOverlap
  (params (OtherActor :type Actor%20Object%20Reference)))

(event EventTick
  (params (DeltaSeconds :type Float%20%28single-precision%29)))

(event Input|ActionEvents|InputActionInteract
  (params (Key :type Key%20Structure :default "None"))
  (:Pressed
    (Utilities|FlowControl|Gate true
      (:Exit
        (Utilities|FlowControl|FlipFlop
          (:A
            (bind _returnvalue (UserInterface|CreateWidget "/Game/LevelOnTheBrink/BP/Picture/Teen_WD.Teen_WD_C"))
            (UserInterface|Viewport|AddtoViewport _returnvalue 0))
          (:B
            (Widget|RemovefromParent _returnvalue)))))))

(fn ConstructionScript)