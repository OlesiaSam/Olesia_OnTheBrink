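; BP_Buttom is a button actor that opens the secret door linked to it.
; Its Interface event finds the Door_secret whose DoorValue matches ButtomValue, calls OpenDoor with the player and blends the view to that door.
; Box overlap enables input and shows Widget_forDoor; all widgets are removed after a short delay or when overlap ends, which also disables input.
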(event OnComponentBeginOverlap(Box)
  (params (OverlappedComponent :type Primitive%20Component%20Object%20Reference) (OtherActor :type Actor%20Object%20Reference) (OtherComp :type Primitive%20Component%20Object%20Reference) (OtherBodyIndex :type Integer) (bFromSweep :type Boolean) (SweepResult :type Hit%20Result%20Structure%20%28by%20ref%29))
  (Input|EnableInput (Game|GetPlayerController 0))
  (bind _returnvalue (UserInterface|CreateWidget "/Game/LevelOnTheBrink/BP/Widget_forDoor.Widget_forDoor_C"))
  (UserInterface|Viewport|AddtoViewport _returnvalue 0)
  (Utilities|FlowControl|Delay 1.0)
  (Viewport|RemoveAllWidgets))

(event OnComponentEndOverlap(Box)
  (params (OverlappedComponent :type Primitive%20Component%20Object%20Reference) (OtherActor :type Actor%20Object%20Reference) (OtherComp :type Primitive%20Component%20Object%20Reference) (OtherBodyIndex :type Integer))
  (Input|DisableInput (Game|GetPlayerController 0))
  (Viewport|RemoveAllWidgets))

(event EventInterface
  (params (Player :type Character%20Object%20Reference))
  ;[1 1 1] Находим все двери из массива
  (bind _outactors (Actor|GetAllActorsOfClass "/Game/LevelOnTheBrink/BP/Door_secret.Door_secret_C"))
  (bind _array_element (Utilities|Array|ForEachLoopwithBreak _outactors :!label _label)
    (:LoopBody
      ;[1 1 1] Определяем какая дверь связана с кнопкой
      (if (== (Variables|/Game/LevelOnTheBrink/BP/Door_secret.Door_secret_C|GetDoor%20Value _array_element) (Variables|Default|GetButtom%20Value))
        ;[1 1 1] Открываем дверь и устанавливам камеру
        (Default|OpenDoor _array_element Player)
        (Game|Player|SetViewTargetwithBlend (Game|GetPlayerController 0) _array_element 0.0 "VTBlend_Linear" 0.0 false)
        (goto _label Break)))))

(fn ConstructionScript)