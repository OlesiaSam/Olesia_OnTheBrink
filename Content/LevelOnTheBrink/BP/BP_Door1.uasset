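; BP_Door1 is a hinged door that the player opens and closes with the Interact action while standing in its trigger box.
; Box overlap enables input for player 0 and briefly shows a TextRender; leaving disables input and hides it.
; Interact plays or reverses a timeline driving the door's relative yaw.
; Each update recomputes DoorOpen from that yaw, so despite its name it is true when rotation is not positive.
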(event OnComponentBeginOverlap(Box)
  (params (OverlappedComponent :type Primitive%20Component%20Object%20Reference) (OtherActor :type Actor%20Object%20Reference) (OtherComp :type Primitive%20Component%20Object%20Reference) (OtherBodyIndex :type Integer) (bFromSweep :type Boolean) (SweepResult :type Hit%20Result%20Structure%20%28by%20ref%29))
  ;[1 1 1] Пересечение игроком коллизии
  (Input|EnableInput (Game|GetPlayerController 0))
  (Rendering|SetVisibility (Variables|Default|GetTextRender) true false)
  (Utilities|FlowControl|Delay 1.0)
  (Rendering|SetVisibility (Variables|Default|GetTextRender) false false))

(event OnComponentEndOverlap(Box)
  (params (OverlappedComponent :type Primitive%20Component%20Object%20Reference) (OtherActor :type Actor%20Object%20Reference) (OtherComp :type Primitive%20Component%20Object%20Reference) (OtherBodyIndex :type Integer))
  ;[1 1 1] Пересечение игроком коллизии
  (Input|DisableInput (Game|GetPlayerController 0))
  (Rendering|SetVisibility (Variables|Default|GetTextRender) false false))

(event EventBeginPlay)

(event Collision|EventActorBeginOverlap
  (params (OtherActor :type Actor%20Object%20Reference)))

(event EventTick
  (params (DeltaSeconds :type Float%20%28single-precision%29)))

(event Input|ActionEvents|InputActionInteract
  (params (Key :type Key%20Structure :default "None"))
  ;[0 0.964 1] Открытие двери с клавиши
  (:Pressed
    (if (Variables|Default|GetDoorOpen)
      (bind _rotate (Timeline|Timeline_DoorOPen Play)
        (:Update
          (Transformation|SetRelativeRotation (Variables|Default|GetDoor) (Math|Rotator|MakeRotator 0.0 0.0 _rotate) false false)
          (Variables|Default|SetDoorOpen (not (> _rotate 0.0)))))
      (else
        (Timeline|Timeline_DoorOPen Reverse)))))

(fn ConstructionScript)